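; Test player pawn for a story playback system that drives scenario and sequence functions.
; BeginPlay and the Fire and Jump inputs call separate test functions, with a debug print shown when player controller 0 possesses the pawn.
; PlayOver stops the sequence player at the end of a page, while the next-page click event is empty.
; Scenario loading by file name and page advance sit in unconnected nodes that never run.
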(event `self.ReceiveBeginPlay`
  (`self.TestFunc`)
  (`KismetSystemLibrary.PrintString` "cnontrol!!!" (== (`self.GetController`) (`GameplayStatics.GetPlayerController` 0)) true (struct :`G` 0.66 :`B` 1.0 :`A` 1.0) 4.0))

(event `InputAction|Fire`
  (params (Key :type "Key Structure"))
  (:`Pressed`
    (`self.TestFuncTwo`)))

(event `OnClickNext`
  ;[1 1 1] 点击开始下一页
)

(event `InputAction|Jump`
  (params (Key :type "Key Structure"))
  (:`Pressed`
    (`self.TestFuncThree`)))

(event `self.ReceiveTick`
  (params (DeltaSeconds :type "Float (single-precision)")))

(event `PlayOver`
  (bind _m_sequenceplayer (`self.m_sequencePlayer`))
  ;[1 1 1] 播放完一页暂停
  (`/Engine/EditorBlueprintResources/StandardMacros.IsValid` _m_sequenceplayer
    (:`Is Valid`
      (`MovieSceneSequencePlayer.Stop` _m_sequenceplayer))))

(fn `UserConstructionScript`)